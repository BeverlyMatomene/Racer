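; Player controller that turns player input into movement, jumping and camera look for the possessed Character.
; Jump and the move axes cast the controlled pawn to Character, then call Jump or feed forward and right input vectors straight to its movement component.
; LookUp and Turn add pitch and yaw input on the controller itself.
; Jump and MoveRight also carry debug screen prints.
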(event `InputAction|Jump`
  (params (Key :type "Key Structure"))
  (:`Pressed`
    (bind _ascharacter (cast `Character` (`self.K2_GetPawn`)))
    (`Character.Jump` _ascharacter)
    (`KismetSystemLibrary.PrintString` "")))

(event `InputAxis|MoveForward`
  (params (AxisValue :type "Float (single-precision)"))
  (bind _ascharacter (cast `Character` (`self.K2_GetPawn`)))
  (`PawnMovementComponent.AddInputVector` (`Pawn.GetMovementComponent` _ascharacter) (* (`self.GetActorForwardVector` _ascharacter) AxisValue) false))

(event `InputAxis|MoveRight`
  (params (AxisValue :type "Float (single-precision)"))
  (bind _ascharacter (cast `Character` (`self.K2_GetPawn`)))
  (`PawnMovementComponent.AddInputVector` (`Pawn.GetMovementComponent` _ascharacter) (* (`self.GetActorRightVector` _ascharacter) AxisValue) false)
  (`KismetSystemLibrary.PrintString` (`KismetStringLibrary.Conv_DoubleToString` AxisValue) true true (struct :`G` 0.66 :`B` 1.0 :`A` 1.0) 0.0))

(event `InputAxis|LookUp`
  (params (AxisValue :type "Float (single-precision)"))
  (`self.AddPitchInput` AxisValue))

(event `InputAxis|Turn`
  (params (AxisValue :type "Float (single-precision)"))
  (`self.AddYawInput` AxisValue))

(fn `UserConstructionScript`)